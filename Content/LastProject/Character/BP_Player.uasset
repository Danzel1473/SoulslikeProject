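; BP_Player is the player character Blueprint, wiring Enhanced Input actions to combat and lock-on behavior.
; The attack input calls Attack only when the battle state is None or Attacking and the character is not falling, so attacks can chain but not start mid-air.
; The lock-on input asks the Lockon component to detect a target.
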(event Input|EnhancedActionEvents|EnhancedInputActionIA_Attack
  (params (ActionValue :type Boolean) (ElapsedSeconds :type Float%20%28double-precision%29) (TriggeredSeconds :type Float%20%28double-precision%29) (InputAction :type Input%20Action%20Object%20Reference :default "/Game/LastProject/Input/InputAction/IA_Attack.IA_Attack"))
  ;[1 1 1] Attack
  (if (and (or (Utilities|Enum|Equal(Enum) (Variables|Default|GetBattleState) "None") (Utilities|Enum|Equal(Enum) (Variables|Default|GetBattleState) "Attacking")) (not (AI|Components|NavMovement|IsFalling (Variables|Character|GetCharacterMovement))))
    (Class|PlayerCharacter|Attack)))

(event Input|EnhancedActionEvents|EnhancedInputActionIA_LockOn
  (params (ActionValue :type Boolean) (ElapsedSeconds :type Float%20%28double-precision%29) (TriggeredSeconds :type Float%20%28double-precision%29) (InputAction :type Input%20Action%20Object%20Reference :default "/Game/LastProject/Input/InputAction/IA_LockOn.IA_LockOn"))
  (Class|LockonComponent|DetectLockonTarget (Variables|Default|GetLockon)))

(event EventBeginPlay)

(event Collision|EventActorBeginOverlap
  (params (OtherActor :type Actor%20Object%20Reference)))

(event EventTick
  (params (DeltaSeconds :type Float%20%28single-precision%29)))

(fn ConstructionScript)
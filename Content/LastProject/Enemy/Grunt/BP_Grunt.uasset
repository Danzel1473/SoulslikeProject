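; BP_Grunt is a Grunt enemy Blueprint that carries an overhead-style HP bar through its HPBarWidget component.
; On BeginPlay it casts the component's widget to WBP_EnemyHPBar and sets itself as that widget's OwnerCharacter.
; Every Tick it billboards the bar by rotating it to look at the first player's camera.
; The overlap event and construction script are empty, and no combat or AI logic appears in these graphs.
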(event EventBeginPlay
  (bind _aswbp_enemy_hpbar (Utilities|Casting|CastToWBP_EnemyHPBar (UserInterface|GetUserWidgetObject (Variables|Default|GetHPBarWidget))))
  (Utilities|IsValid _aswbp_enemy_hpbar
    (:Is%20Valid
      (Variables|/Game/LastProject/ui/WBP_EnemyHPBar.WBP_EnemyHPBar_C|SetOwnerCharacter _aswbp_enemy_hpbar self))))

(event Collision|EventActorBeginOverlap
  (params (OtherActor :type Actor%20Object%20Reference)))

(event EventTick
  (params (DeltaSeconds :type Float%20%28single-precision%29))
  (bind _hpbarwidget (Variables|Default|GetHPBarWidget))
  (Transformation|SetWorldRotation _hpbarwidget (Math|Rotator|FindLookatRotation (Transformation|GetWorldLocation _hpbarwidget) (Camera|GetCameraLocation (Game|GetPlayerCameraManager 0))) false false))

(fn ConstructionScript)